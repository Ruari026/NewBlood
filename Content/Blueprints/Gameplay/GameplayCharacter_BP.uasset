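; Gameplay character Blueprint that wears the suspect model picked on the character select screen.
; On BeginPlay, the locally controlled instance reads PlayerSuspectType from the GameInfoInstance and passes it to ChangeModel.
; ChangeModel swaps the SuspectMesh child actor class between colored suspect Blueprints, defaulting to red.
; Tick sets IsWalking on the child suspect's animation instance from whether movement velocity is nonzero.
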(event Custom|ChangeModel
  (params (NewModel :type String))
  (bind _suspectmesh (Variables|Default|GetSuspectMesh))
  (switch string NewModel
    (:Default
      (ChildActorComponent|SetChildActorClass _suspectmesh "/Game/Blueprints/AllLevels/Suspects/RedSuspect_BP.RedSuspect_BP_C" :!label _label))
    (:Red
      (goto _label))
    (:Blue
      (ChildActorComponent|SetChildActorClass _suspectmesh "/Game/Blueprints/AllLevels/Suspects/BlueSuspect_BP.BlueSuspect_BP_C"))
    (:Yellow
      (ChildActorComponent|SetChildActorClass _suspectmesh "/Game/Blueprints/AllLevels/Suspects/YellowSuspect_BP.YellowSuspect_BP_C"))
    (:Green
      (ChildActorComponent|SetChildActorClass _suspectmesh "/Game/Blueprints/AllLevels/Suspects/GreenSuspect_BP.GreenSuspect_BP_C"))))

(event EventBeginPlay
  ;[1 1 1] Player Mesh Selected Based On The Character Select Screen
  (if (Pawn|IsLocallyControlled)
    (bind _asgame_info_instance (Utilities|Casting|CastToGameInfoInstance (Game|GetGameInstance)))
    (CallFunction|ChangeModel (Variables|/Game/Blueprints/AllLevels/GameInfoInstance.GameInfoInstance_C|GetPlayerSuspectType _asgame_info_instance))))

(event EventTick
  (params (DeltaSeconds :type Float%20%28single-precision%29))
  (bind _asbase_suspect_bp (Utilities|Casting|CastToBaseSuspect_BP (Variables|/Script/Engine.ChildActorComponent|GetChildActor (Variables|Default|GetSuspectMesh))))
  (if (> (Math|Vector|VectorLength (Variables|/Script/Engine.MovementComponent|GetVelocity (Variables|Character|GetCharacterMovement))) 0.0)
    (bind _assuspect_anim_controller (Utilities|Casting|CastToSuspectAnimController (Components|SkeletalMesh|GetAnimInstance (Variables|/Game/Blueprints/AllLevels/Suspects/BaseSuspect_BP.BaseSuspect_BP_C|GetSuspectMesh _asbase_suspect_bp))))
    (Variables|/Game/Animation/Suspects/SuspectAnimController.SuspectAnimController_C|SetIsWalking _assuspect_anim_controller true)
    (else
      (bind _assuspect_anim_controller_2 (Utilities|Casting|CastToSuspectAnimController (Components|SkeletalMesh|GetAnimInstance (Variables|/Game/Blueprints/AllLevels/Suspects/BaseSuspect_BP.BaseSuspect_BP_C|GetSuspectMesh _asbase_suspect_bp))))
      (Variables|/Game/Animation/Suspects/SuspectAnimController.SuspectAnimController_C|SetIsWalking _assuspect_anim_controller_2 false))))

(fn ConstructionScript)