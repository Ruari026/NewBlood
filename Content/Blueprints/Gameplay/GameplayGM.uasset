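; GameplayGM is a game mode that sets up a murder scenario when a player login brings the GameplayPC count to exactly three.
; It randomly picks and stores a murderer from the PlayerControllers and a weapon from the InteractableWeapon actors in the world.
; It then passes a hardcoded victim name and the weapon's damage type, as murder method, to the VictimBase_BP actor through SetVictimDetails.
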(event EventBeginPlay)

(event EventTick
  (params (DeltaSeconds :type Float%20%28single-precision%29)))

(event EventPostLogin
  (params (NewPlayer :type Player%20Controller%20Object%20Reference))
  ;[1 1 1] Checking That All Players Are Connected
  (bind _outactors (Actor|GetAllActorsOfClass "/Game/Blueprints/Gameplay/GameplayPC.GameplayPC_C"))
  (if (== (Utilities|Array|Length _outactors) 3)
    ;[1 1 1] Setup Murder Scenario - Murderer
    (bind _outactors_2 (Actor|GetAllActorsOfClass "/Script/Engine.PlayerController"))
    (bind _result (Math|Integer|DecrementInt (Utilities|Array|Length _outactors_2))
      (:%20%20
        (Variables|Default|SetPickedMurderer (Utilities|Array|Get(acopy) _outactors_2 (Math|Random|RandomIntegerinRange 0 _result)))
        ;[1 1 1] Setup Murder Scenario - Weapon
        (bind _outactors_3 (Actor|GetAllActorsOfClass "/Script/NewBlood.InteractableWeapon"))
        (bind _result_2 (Math|Integer|DecrementInt (Utilities|Array|Length _outactors_3))
          (:%20%20
            (bind _output_get (Variables|Default|SetPickedWeapon (Utilities|Array|Get(acopy) _outactors_3 (Math|Random|RandomIntegerinRange 0 _result_2))))
            ;[1 1 1] Broadcasting Weapon Info
            (bind _returnvalue (Actor|GetActorOfClass "/Game/Blueprints/Gameplay/Victims/VictimBase_BP.VictimBase_BP_C"))
            (Default|SetVictimDetails _returnvalue "Mrs NuBlud" (Variables|/Script/NewBlood.InteractableWeapon|GetdamageType _output_get))))))))

(fn ConstructionScript)